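; BP_Checkpoint is a numbered checkpoint that grants boost to the third-person character the first time it enters the trigger.
; On overlap, it checks CheckpointNum (1 to 3) against the matching flag on BP_ThirdPersonCharacter, calls AddBoost with GainBoost, then sets that flag.
; The once-only state lives on the character, so the checkpoint stays active.
; Unconnected leftover nodes for hiding the actor and boosting BP_Hoverboard never run.
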(event `self.CheckpointTrigger.OnComponentBeginOverlap`
  (params (OverlappedComponent :type "PrimitiveComponent Object Reference") (OtherActor :type "Actor Object Reference") (OtherComp :type "PrimitiveComponent Object Reference") (OtherBodyIndex :type Integer) (bFromSweep :type Boolean) (SweepResult :type "HitResult Structure (by ref)"))
  (bind _asbp_third_person_character (cast `/Game/ThirdPerson/Blueprints/BP_ThirdPersonCharacter` OtherActor))
  (if (or (and (== (`self.CheckpointNum`) 1) (== (`/Game/ThirdPerson/Blueprints/BP_ThirdPersonCharacter.Checkpoint1` _asbp_third_person_character) false)) (and (== (`self.CheckpointNum`) 2) (== (`/Game/ThirdPerson/Blueprints/BP_ThirdPersonCharacter.Checkpoint2` _asbp_third_person_character) false)) (and (== (`self.CheckpointNum`) 3) (== (`/Game/ThirdPerson/Blueprints/BP_ThirdPersonCharacter.Checkpoint3` _asbp_third_person_character) false)))
    (`/Game/ThirdPerson/Blueprints/BP_ThirdPersonCharacter.AddBoost` _asbp_third_person_character (`self.Gain Boost`))
    (switch `int` (`self.CheckpointNum`)
      (:`1`
        (set `/Game/ThirdPerson/Blueprints/BP_ThirdPersonCharacter.Checkpoint1` true _asbp_third_person_character))
      (:`2`
        (set `/Game/ThirdPerson/Blueprints/BP_ThirdPersonCharacter.Checkpoint2` true _asbp_third_person_character))
      (:`3`
        (set `/Game/ThirdPerson/Blueprints/BP_ThirdPersonCharacter.Checkpoint3` true _asbp_third_person_character)))))

(fn `UserConstructionScript`)